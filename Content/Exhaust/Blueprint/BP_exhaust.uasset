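; BP_exhaust is an exhaust effect actor combining a mesh, a Cascade particle system and a point light, configured in the construction script.
; It creates a dynamic instance of MT_Exhaust_Master on the mesh to set color and main animation speed.
; The same color tints the particle sparks and the light, while a separate parameter scales smoke emission.
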(fn ConstructionScript
  (bind _fx_exhaust (Variables|Default|GetFX_Exhaust))
  (bind _color (Variables|Default|GetColor))
  ;[1 1 1] Create Dynamic Material Instance and Store in Variable
  (bind _returnvalue (Rendering|Material|CreateDynamicMaterialInstance (Variables|Default|GetExhaustMesh) 0 "/Game/Exhaust/Material/MT_Exhaust_Master.MT_Exhaust_Master" :!class /Script/Engine.PrimitiveComponent))
  (Variables|Default|SetMatExhaust _returnvalue)
  (Rendering|Material|SetVectorParameterValue (Variables|Default|GetMatExhaust) "Color" _color :!class /Script/Engine.MaterialInstanceDynamic) ; Set Color in Material
  (Effects|Components|ParticleSystem|SetColorParameter _fx_exhaust "SparksColor" _color) ; Set Color in Cascade Params for Sparks
  (Rendering|Material|SetScalarParameterValue (Variables|Default|GetMatExhaust) "MainSpeed" (Variables|Default|GetMainSpeed) :!class /Script/Engine.MaterialInstanceDynamic) ; Control Speed
  (Rendering|Components|Light|SetLightColor (Variables|Default|GetPointLight) _color true) ; Set Color of Light
  (Effects|Components|ParticleSystem|SetFloatParameter _fx_exhaust "SmokeEmit" (Variables|Default|GetSmokeEmit)) ; Rate Scale for Smoke Emit
)